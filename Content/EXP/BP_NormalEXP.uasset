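; BP_NormalEXP is an experience pickup actor that grants its EXP value to the player character.
; BeginPlay caches the player pawn as a Grim_Chara reference.
; Each Magnet call moves the pickup a step toward the player with VInterpTo, teleport and sweep off.
; EXPGain passes EXP to the player's GainEXP and destroys the actor; neither event is triggered within this Blueprint.
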(event Custom|EXP%20Gain
  (Default|GainEXP (Variables|Default|GetPlayer) (Variables|Default|GetEXP))
  (Actor|DestroyActor))

(event Custom|Magnet
  (Transformation|SetActorLocation (Math|Interpolation|VInterpTo (Transformation|GetActorLocation) (Transformation|GetActorLocation (Variables|Default|GetPlayer)) (Utilities|Time|GetWorldDeltaSeconds) 4.0) false false))

(event EventBeginPlay
  (bind _asgrim_chara (Utilities|Casting|CastToGrim_Chara (Game|Player|GetPlayerPawn 0)))
  (Variables|Default|SetPlayer _asgrim_chara))

(fn ConstructionScript)